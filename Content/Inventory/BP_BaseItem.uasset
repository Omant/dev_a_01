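; BP_BaseItem is a base item Blueprint for the inventory, carrying an ItemData struct that describes the item.
; Its construction script rebuilds ItemData with the actor's own class in the class field and keeps the other fields, so the data always references the Blueprint it belongs to.
; The event graph holds only disabled default events, so it adds no runtime behavior.
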(fn `UserConstructionScript`
  (bind (_itemdata_itemtype _itemdata_name _itemdata_description _itemdata_image _itemdata_itemclass _itemdata_itemslot _itemdata_weight _itemdata_amount _itemdata_stackable _itemdata_itemindex) (break `/Game/Inventory/ItemData` (`self.ItemData`)))
  (`parent.UserConstructionScript`)
  (set `self.ItemData` (make `/Game/Inventory/ItemData` _itemdata_itemtype _itemdata_name _itemdata_description _itemdata_image (`GameplayStatics.GetObjectClass` self) _itemdata_itemslot _itemdata_weight _itemdata_amount _itemdata_stackable _itemdata_itemindex)))